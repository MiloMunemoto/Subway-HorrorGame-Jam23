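; BP_TrashBagWithRat is a trash bag prop with a trigger box that reacts when the first-person character walks into it.
; The overlap checks the character's TriggersWalked counter: at two it prints a "BOOOH" debug string and stops TrashaBagCue after a delay.
; Otherwise it stops the cue at once, then increments and prints the counter.
; A PlayAnimation node is present but never runs.
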(event `self.TriggerBox.OnComponentBeginOverlap`
  (params (OverlappedComponent :type "PrimitiveComponent Object Reference") (OtherActor :type "Actor Object Reference") (OtherComp :type "PrimitiveComponent Object Reference") (OtherBodyIndex :type Integer) (bFromSweep :type Boolean) (SweepResult :type "HitResult Structure (by ref)"))
  (bind _asbp_first_person_character (cast `/Game/FirstPerson/Blueprints/BP_FirstPersonCharacter` OtherActor))
  (bind _triggerswalked (`/Game/FirstPerson/Blueprints/BP_FirstPersonCharacter.TriggersWalked` _asbp_first_person_character))
  (if (== _triggerswalked 2)
    (`KismetSystemLibrary.PrintString` "BOOOH")
    (`KismetSystemLibrary.Delay` 2.0)
    (`AudioComponent.Stop` (`self.TrashaBag_Cue`))
    (else
      (`AudioComponent.Stop` (`self.TrashaBag_Cue`))
      (bind _result (`/Engine/EditorBlueprintResources/StandardMacros.IncrementInt` _triggerswalked)
        (:`  `
          (`KismetSystemLibrary.PrintString` (`KismetStringLibrary.Conv_IntToString` _result)))))))

(fn `UserConstructionScript`)