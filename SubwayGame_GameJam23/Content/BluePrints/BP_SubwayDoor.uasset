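; BP_SubwayDoor is a subway door that the player opens with the interaction input while standing in its trigger.
; Trigger overlap by the first-person character enables input and adds the interaction mapping context; leaving disables input.
; Interacting slides the door sideways with MoveComponentTo, waits briefly, then slides it back, guarded by IsDoorOpening.
; Each move plays the same opening sound from an offset and stops it when the move completes.
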(event `EnhancedInput|/Game/BluePrints/IA_Interaction`
  (params (ActionValue :type Boolean) (ElapsedSeconds :type "Float (double-precision)") (TriggeredSeconds :type "Float (double-precision)") (InputAction :type "InputAction Object Reference" :default "/Game/BluePrints/IA_Interaction.IA_Interaction"))
  (bind _subwaydoor (`self.SubwayDoor`))
  (bind _relativelocation (`SceneComponent.RelativeLocation` _subwaydoor))
  (:`Started`
    (if (not (`self.IsDoorOpening`))
      (set `self.IsDoorOpening` true)
      (bind _returnvalue (`GameplayStatics.SpawnSound2D` (`self.DoorOpening`) 1.0 1.0 1.7 null))
      (set `self.OpeningDoor` _returnvalue)
      (`KismetSystemLibrary.MoveComponentTo` _subwaydoor (+ _relativelocation (0.0 150.0 0.0)) (struct) true false 2.0)
      (`AudioComponent.Stop` (`self.OpeningDoor`))
      (`KismetSystemLibrary.Delay` 2.0)
      (bind _returnvalue_2 (`GameplayStatics.SpawnSound2D` (`self.DoorOpening`) 1.0 1.0 1.7 null))
      (set `self.ClosingDoor` _returnvalue_2)
      (`KismetSystemLibrary.MoveComponentTo` _subwaydoor (+ _relativelocation (0.0 -150.0 0.0)) (struct) true false 2.0)
      (`AudioComponent.Stop` (`self.ClosingDoor`))
      (set `self.IsDoorOpening` false))))

(event `self.Trigger.OnComponentBeginOverlap`
  (params (OverlappedComponent :type "PrimitiveComponent Object Reference") (OtherActor :type "Actor Object Reference") (OtherComp :type "PrimitiveComponent Object Reference") (OtherBodyIndex :type Integer) (bFromSweep :type Boolean) (SweepResult :type "HitResult Structure (by ref)"))
  (bind _asbp_first_person_character (cast `/Game/FirstPerson/Blueprints/BP_FirstPersonCharacter` OtherActor))
  (`self.EnableInput` (`GameplayStatics.GetPlayerController` 0))
  (bind _asplayer_controller (cast `PlayerController` (`Pawn.GetController` _asbp_first_person_character)))
  (`/Engine/EditorBlueprintResources/StandardMacros.IsValid` _asplayer_controller
    (:`Is Valid`
      (`EnhancedInputSubsystemInterface.AddMappingContext` (pcsubsystem `EnhancedInputLocalPlayerSubsystem` _asplayer_controller) "/Game/BluePrints/IM_Interaction.IM_Interaction" 0 (struct)))))

(event `self.Trigger.OnComponentEndOverlap`
  (params (OverlappedComponent :type "PrimitiveComponent Object Reference") (OtherActor :type "Actor Object Reference") (OtherComp :type "PrimitiveComponent Object Reference") (OtherBodyIndex :type Integer))
  (`self.DisableInput` (`GameplayStatics.GetPlayerController` 0)))

(fn `UserConstructionScript`)