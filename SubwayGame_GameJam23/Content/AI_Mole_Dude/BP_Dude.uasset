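; BP_Dude is an enemy AI that chases the first-person player and restarts the level on contact.
; PawnSensing starts an AI MoveTo toward a seen player and sets CanSeePlayer, which a retriggerable half-second delay clears once sightings stop.
; Player overlap with Trigger prints a message, plays a scream, waits briefly, then reloads the current level.
; A random wandering branch for when the player is unseen exists but is never executed.
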(event `self.PawnSensing.OnSeePawn`
  (params (Pawn :type "Pawn Object Reference"))
  (bind _asbp_first_person_character (cast `/Game/FirstPerson/Blueprints/BP_FirstPersonCharacter` Pawn))
  (`|ExecutionSequence`
    (:`then_0`
      (set `self.CanSeePlayer` true)
      (`|AIMoveTo` self (0.0 0.0 0.0) _asbp_first_person_character))
    (:`then_1`
      (`KismetSystemLibrary.RetriggerableDelay` 0.5)
      (set `self.CanSeePlayer` false))))

(event `self.Trigger.OnComponentBeginOverlap`
  (params (OverlappedComponent :type "PrimitiveComponent Object Reference") (OtherActor :type "Actor Object Reference") (OtherComp :type "PrimitiveComponent Object Reference") (OtherBodyIndex :type Integer) (bFromSweep :type Boolean) (SweepResult :type "HitResult Structure (by ref)"))
  (cast `/Game/FirstPerson/Blueprints/BP_FirstPersonCharacter` OtherActor)
  (`KismetSystemLibrary.PrintString` "YOU FUCKED UP")
  (`GameplayStatics.PlaySoundAtLocation` "/Game/AI_Mole_Dude/Sounds/scream_cue.scream_cue" (`self.K2_GetActorLocation`) (struct) 1.0 1.0 0.0 null null null null)
  (`KismetSystemLibrary.Delay` 1.5)
  (bind _returnvalue (`GameplayStatics.GetCurrentLevelName` true))
  (`GameplayStatics.OpenLevel` (`KismetStringLibrary.Conv_StringToName` _returnvalue)))

(fn `UserConstructionScript`)