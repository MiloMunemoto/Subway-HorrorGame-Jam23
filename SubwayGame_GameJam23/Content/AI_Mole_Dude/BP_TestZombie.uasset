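; BP_TestZombie is a test zombie AI pawn that chases the first-person player character when its PawnSensing component sees it.
; Each sighting sets CanSeePlayer and issues an AI MoveTo toward the player, while a retriggerable half-second delay clears the flag once sightings stop.
; A random wander routine to reachable nearby points, gated on CanSeePlayer, is present but unconnected, so it never runs.
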(event `self.ReceiveActorBeginOverlap`
  (params (OtherActor :type "Actor Object Reference")))

(event `self.ReceiveTick`
  (params (DeltaSeconds :type "Float (single-precision)")))

(event `self.PawnSensing.OnSeePawn`
  (params (Pawn :type "Pawn Object Reference"))
  (bind _asbp_first_person_character (cast `/Game/FirstPerson/Blueprints/BP_FirstPersonCharacter` Pawn))
  (`|ExecutionSequence`
    (:`then_0`
      (set `self.CanSeePlayer` true)
      (`|AIMoveTo` self (0.0 0.0 0.0) _asbp_first_person_character))
    (:`then_1`
      (`KismetSystemLibrary.RetriggerableDelay` 0.5)
      (set `self.CanSeePlayer` false))))

(fn `UserConstructionScript`)